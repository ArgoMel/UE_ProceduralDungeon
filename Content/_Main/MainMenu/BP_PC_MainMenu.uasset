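; BP_PC_MainMenu is the main menu player controller that handles hosting and joining multiplayer sessions.
; HostGame creates an advanced session carrying the game name and max player count as extra settings, then opens the Test level as a listen server on success.
; JoinGameBP joins a supplied session search result.
; Both paths only print a message on failure, and BeginPlay, Tick and the construction script are empty.
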(event `self.HostGame`
  (params (GameName :type String) (Players :type Integer))
  (`CreateSessionCallbackProxyAdvanced.CreateAdvancedSession` (`|MakeArray` (`AdvancedSessionsLibrary.MakeLiteralSessionPropertyString` "GameName" GameName) (`AdvancedSessionsLibrary.MakeLiteralSessionPropertyInt` "MaxPlayers" Players)) self
    (:`OnSuccess`
      (`GameplayStatics.OpenLevelBySoftObjectPtr` "/Game/_Main/Maps/Test.Test" true "?listen"))
    (:`OnFailure`
      (`KismetSystemLibrary.PrintString` "Failed Create Session"))))

(event `/Game/_Main/MainMenu/INT_MainMenuBP.JoinGameBP`
  (params (SessionResult :type "BlueprintSessionResult Structure"))
  (`JoinSessionCallbackProxy.JoinSession` self SessionResult
    (:`OnFailure`
      (`KismetSystemLibrary.PrintString` "Join session failsd"))))

(fn `UserConstructionScript`)